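; Clickable interface actor that lets the player grab physics components with the left mouse button.
; Pressing runs a Visibility line trace built from InterfaceCamera and passes the hit component to a PhysicsHandle without checking the hit; releasing drops it.
; Mouse movement updates the handle target, but location and forward vector appear swapped in the math, so the target resolves to just the camera's forward vector.
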(event `Key|LeftMouseButton`
  (params (Key :type "Key Structure"))
  (bind _interface_camera (`self.interface Camera`))
  (bind _returnvalue (`SceneComponent.GetForwardVector` _interface_camera))
  (:`Pressed`
    (bind _outhit (`KismetSystemLibrary.LineTraceSingle` _returnvalue (+ (* (`SceneComponent.K2_GetComponentLocation` _interface_camera) 246.0) _returnvalue) "TraceTypeQuery1"))
    (if true
      (bind (_bblockinghit _binitialoverlap _time _distance _location _impactpoint _normal _impactnormal _physmat _hitactor _hitcomponent) (`GameplayStatics.BreakHitResult` _outhit))
      (`PhysicsHandleComponent.GrabComponentAtLocation` (`self.PhysicsHandle`) _hitcomponent "None" (`SceneComponent.K2_GetComponentLocation` _hitcomponent))))
  (:`Released`
    (`PhysicsHandleComponent.ReleaseComponent` (`self.PhysicsHandle`))))

(event `InputVectorAxis|Mouse2D`
  (params (AxisValue :type "Vector Structure"))
  (bind _interface_camera (`self.interface Camera`))
  (`PhysicsHandleComponent.SetTargetLocation` (`self.PhysicsHandle`) (+ (* (`SceneComponent.K2_GetComponentLocation` _interface_camera) 0.0) (`SceneComponent.GetForwardVector` _interface_camera))))

(fn `UserConstructionScript`)